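; Experimental player Character Blueprint that sets up a basic HUD and handles sprint, crouch and aim input.
; On BeginPlay it creates the idle crosshair and health bar widgets and adds them to the viewport.
; Sprint raises max walk speed while held, Crouch toggles between crouched and standing, and Aim sets an IsAiming flag while held.
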(event EventBeginPlay
  (bind _returnvalue (UserInterface|CreateWidget "/Game/HUD/WBP_CrosshairIdle.WBP_CrosshairIdle_C"))
  (UserInterface|Viewport|AddtoViewport _returnvalue 0)
  (bind _returnvalue_2 (UserInterface|CreateWidget "/Game/HUD/WBP_HealthBar.WBP_HealthBar_C"))
  (UserInterface|Viewport|AddtoViewport _returnvalue_2 0))

(event Collision|EventActorBeginOverlap
  (params (OtherActor :type Actor%20Object%20Reference)))

(event EventTick
  (params (DeltaSeconds :type Float%20%28single-precision%29)))

(event Input|ActionEvents|InputActionSprint
  (params (Key :type Key%20Structure))
  (bind _charactermovement (Variables|Character|GetCharacterMovement))
  (:Pressed
    (Variables|/Script/Engine.CharacterMovementComponent|SetMaxWalkSpeed _charactermovement 8e+02))
  (:Released
    (Variables|/Script/Engine.CharacterMovementComponent|SetMaxWalkSpeed _charactermovement 6e+02)))

(event Input|ActionEvents|InputActionCrouch
  (params (Key :type Key%20Structure))
  (:Pressed
    (bind _output_get (Variables|Default|SetIsCrouched (not (Variables|Default|GetIsCrouched))))
    (if _output_get
      (Character|Crouch)
      (else
        (Character|UnCrouch)))))

(event Input|ActionEvents|InputActionAim
  (params (Key :type Key%20Structure))
  (:Pressed
    (Variables|Default|SetIsAiming true))
  (:Released
    (Variables|Default|SetIsAiming false)))

(fn ConstructionScript)